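; BP_TRTCPlayer is a test actor that plays an RTMP live stream on a cube in the level.
; On BeginPlay it constructs a TRTCLivePlayer, starts a hardcoded stream URL, and puts a dynamic instance of MParent on the cube.
; After a short fixed delay, it binds the player's render target texture to the material's Tex parameter.
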(event `self.ReceiveBeginPlay`
  (bind _trtcliveplayer (`self.TRTCLivePlayer`))
  (bind _returnvalue (`|GenericCreateObject` "/Script/TRTCPlugin.TRTCLivePlayer"))
  (set `self.TRTCLivePlayer` _returnvalue)
  (`TRTCLivePlayer.StartPlay` _trtcliveplayer "rtmp://play.psyai.com/psyai1720507015rN/live1720507015rN?auth_key=1721803016-0-0-cb0825528eb5dc7856e852120e1fb20e")
  (bind _returnvalue_2 (`KismetMaterialLibrary.CreateDynamicMaterialInstance` (`self.M_Parent`)))
  (bind _output_get (set `self.M_Ins` _returnvalue_2))
  (`PrimitiveComponent.SetMaterial` (`self.Cube`) 0 _output_get)
  (`KismetSystemLibrary.Delay` 2.0)
  (`MaterialInstanceDynamic.SetTextureParameterValue` (`self.M_Ins`) "Tex" (`TRTCLivePlayer.RenderTargetTexture` _trtcliveplayer)))

(fn `UserConstructionScript`)